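; Main menu player controller that sets up the menu screen, cursor and music.
; On BeginPlay it caches the BP_GameCore game instance, creates and focuses BPW_MainMenu with Game-and-UI input, and plays menu music as a 2D sound.
; The music is resolved from a data table row through a GetSoundDataCue helper.
; Escape exits the options menu held by the game instance when that menu is visible.
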(event EventBeginPlay
  (bind _returnvalue (Game|GetPlayerController 0))
  (Utilities|FlowControl|Sequence
    (:then_0
      (Input|SetInputModeGameandUI (Game|GetPlayerController 0) 0 "DoNotLock" false)
      (bind _asbp_game_core (Utilities|Casting|CastToBP_GameCore (Game|GetGameInstance)))
      (Variables|Private|SetGameCore_REF _asbp_game_core))
    (:then_1
      (Input|EnableInput (Game|GetPlayerController 0)))
    (:then_2
      (Utilities|FlowControl|Sequence
        (:then_0
          (bind _returnvalue_2 (UserInterface|CreateWidget "/Game/Blueprints/WidgetBlueprints/Menus/BPW_MainMenu.BPW_MainMenu_C" _returnvalue))
          (UserInterface|Viewport|AddtoViewport _returnvalue_2 0)
          (Input|SetInputModeGameandUI _returnvalue _returnvalue_2 "LockInFullscreen" false)
          (Variables|/Script/Engine.PlayerController|SetbShowMouseCursor _returnvalue true))
        (:then_1
          (bind _soundcue (CallFunction|GetSoundDataCue (Variables|Inspector|GetMainMenuMusic)))
          (Audio|PlaySound2D _soundcue 1.0 1.0 0.0 0 0))))))

(event Input|KeyboardEvents|Escape
  (params (Key :type Key%20Structure :default "None"))
  (bind _gamecore_ref (Variables|Private|GetGameCore_REF))
  (bind _optionsmenu_ref (Variables|/Game/Blueprints/GameInstances/BP_GameCore.BP_GameCore_C|GetOptionsMenu_REF _gamecore_ref))
  (:Pressed
    (Development|PrintString "Escape")
    (Utilities|IsValid _optionsmenu_ref
      (:Is%20Valid
        (if (Widget|IsVisible _optionsmenu_ref)
          (Default|ExitOptionsMenu _optionsmenu_ref))))))

(fn ConstructionScript)

(fn GetSoundDataCue
  (params (SoundData :type Data%20Table%20Row%20Handle%20Structure))
  (bind (_datatable _rowname) (Utilities|Struct|BreakDataTableRowHandle SoundData))
  (bind _returnvalue (Utilities|GetDataTableRow _datatable _rowname)
    (:then
      _)
    (:RowNotFound
      _))
  (return (Utilities|Struct|BreakAudioStruct _returnvalue)))