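; BP_RunPlayerController is the player controller for the run character, handling sideways movement input and game over.
; On BeginPlay it caches the controlled BP_RunCharacter and binds an event to its death dispatcher.
; The Move Right / Left axis moves the character along its right vector only while it is alive.
; CallGameOver forwards to GameOver on BP_RunGameMode.
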(event Custom|CallGameOver
  ;[1 0 0.7962] Gloabal Management
  (bind _asbp_run_game_mode (Utilities|Casting|CastToBP_RunGameMode (Game|GetGameMode)))
  (Default|GameOver _asbp_run_game_mode))

(event EventBeginPlay
  ;[1 1 1] Init
  (bind _asbp_run_character (Utilities|Casting|CastToBP_RunCharacter (Pawn|GetControlledPawn)))
  (bind _output_get (Variables|Public|SetRunCharacter _asbp_run_character))
  (EventDispatchers|BindEventtoEventPlayerDeath _output_get (EventDispatchers|CreateEvent :!event Custom|CallGameOver)))

(event Input|AxisEvents|InputAxisMoveRight/Left
  (params (AxisValue :type Float%20%28single-precision%29))
  ;[1 0 0.1333] Character Movements Inputs
  (bind _runcharacter (Variables|Public|GetRunCharacter)
    (:then
      (if (Variables|/Game/Blueprints/Actors/BP_RunCharacter.BP_RunCharacter_C|GetIsAlive _runcharacter)
        (Pawn|Input|AddMovementInput _runcharacter (Transformation|GetActorRightVector _runcharacter) AxisValue false)))
    (:else)))

(fn ConstructionScript)