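; BP_RunPlayerControllerScript is a player controller that toggles the pause menu during a run.
; The Pause input action calls SetGamePauseState, which creates BPW_PauseMenu on first use and caches it.
; When unpaused, it adds the menu to the viewport, pauses the game, shows the cursor and switches to Game and UI input.
; When already paused, it hands off to the menu's Resume function.
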(event EventBeginPlay)

(event EventTick
  (params (DeltaSeconds :type Float%20%28single-precision%29)))

(event Input|ActionEvents|InputActionPause
  (params (Key :type Key%20Structure :default "None"))
  (:Pressed
    (Development|PrintString "Pause")
    (CallFunction|SetGamePauseState)))

(fn ConstructionScript)

(fn SetGamePauseState
  (Utilities|IsValid (Variables|Private|Get_pauseMenu_REF)
    (:Is%20Valid
      _)
    (:Is%20Not%20Valid
      (bind _returnvalue (UserInterface|CreateWidget "/Game/Blueprints/WidgetBlueprints/Menus/BPW_PauseMenu.BPW_PauseMenu_C"))
      (Variables|Private|Set_pauseMenu_REF _returnvalue)))
  (if (Game|IsGamePaused)
    (Default|Resume (Variables|Private|Get_pauseMenu_REF))
    (else
      (UserInterface|Viewport|AddtoViewport (Variables|Private|Get_pauseMenu_REF) 20)
      (Game|SetGamePaused true)
      (Variables|Default|SetbShowMouseCursor true)
      (Input|SetInputModeGameandUI self 0 "DoNotLock" true))))