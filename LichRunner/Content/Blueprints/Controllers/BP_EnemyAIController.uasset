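; AI controller for enemy characters that starts their behavior tree and exposes setters for its blackboard state.
; On BeginPlay, InitBehaviourTree prints a debug message with the Instigator's name, runs BT_AIEnemy, then applies BB_AIEnemy.
; The SetEnemyState and SetFollowActor events write the EnemyState enum and FollowActor object keys to the Blackboard.
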(event Custom|SetEnemyState
  (params (EnemyState :type EnumEnemyState%20Enum :default "NewEnumerator0"))
  (AI|Components|Blackboard|SetValueasEnum (Variables|Default|GetBlackboard) (Utilities|Name|MakeLiteralName "EnemyState") EnemyState))

(event Custom|SetFollowActor
  (params (FollowActor :type Actor%20Object%20Reference))
  (AI|Components|Blackboard|SetValueasObject (Variables|Default|GetBlackboard) (Utilities|Name|MakeLiteralName "FollowActor") FollowActor))

(event EventBeginPlay
  (Utilities|FlowControl|Sequence
    (:then_0
      (CallFunction|InitBehaviourTree))))

(fn ConstructionScript)

(fn InitBehaviourTree
  (Development|PrintString (Utilities|String|Append (Utilities|GetDisplayName (Variables|Actor|GetInstigator)) "InitTree"))
  (AI|RunBehaviorTree "/Game/Blueprints/Actors/Characters/BT_AIEnemy.BT_AIEnemy")
  (Class|AIController|UseBlackboard "/Game/Blueprints/Actors/Characters/BB_AIEnemy.BB_AIEnemy"))