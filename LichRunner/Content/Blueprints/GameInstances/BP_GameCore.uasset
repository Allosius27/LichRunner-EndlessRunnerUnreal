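; BP_GameCore, kept with the game instances, provides lazily created, cached access to the shared options menu and requester widgets.
; GetOptionsMenuInstance creates the menu and loads its settings if the cached reference is invalid, then adds it to the viewport on every call.
; GetRequester returns the cached requester, clearing its Yes and No dispatcher bindings only when it creates a new one.
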(fn GetOptionsMenuInstance
  (Utilities|IsValid (Variables|Public|GetOptionsMenu_REF)
    (:Is%20Valid
      _)
    (:Is%20Not%20Valid
      (bind _returnvalue (UserInterface|CreateWidget "/Game/Blueprints/WidgetBlueprints/Menus/BPW_OptionsMenu.BPW_OptionsMenu_C"))
      (bind _output_get (Variables|Public|SetOptionsMenu_REF _returnvalue))
      (Default|LoadSettings _output_get)))
  (UserInterface|Viewport|AddtoViewport (Variables|Public|GetOptionsMenu_REF) 30))

(fn GetRequester
  (Variables|Private|GetRequester_REF
    (:then
      _)
    (:else
      (bind _returnvalue (Game|ConstructObjectfromClass "/Game/Blueprints/WidgetBlueprints/Menus/BPW_Requester.BPW_Requester_C"))
      (Variables|Private|SetRequester_REF _returnvalue)
      (EventDispatchers|UnbindallEventsfromDispatchYes (Variables|Private|GetRequester_REF))
      (EventDispatchers|UnbindallEventsfromDispatchNo (Variables|Private|GetRequester_REF))))
  (return (Variables|Private|GetRequester_REF)))