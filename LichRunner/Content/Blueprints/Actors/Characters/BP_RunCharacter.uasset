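; Player character for a runner game: a rider on an armoured horse that moves forward automatically while alive.
; Pickup adds to yellow or blue coin totals by type and prints the new total.
; A Hit triggers Death, which disables input, plays death animations on the rider and each horse part's anim instance, spawns an emitter and random sound, hides the meshes after a delay, and calls the player-death event.
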(event Custom|MoveForward
  ;[1 0.317 0] Actions
  (if (Variables|Public|GetIsAlive)
    (Pawn|Input|AddMovementInput (Transformation|GetActorForwardVector) 1.0 false)))

(event Custom|Death
  ;[1 0.317 0] Actions
  (Utilities|FlowControl|Sequence
    (:then_0
      (Variables|Public|SetIsAlive false))
    (:then_1
      (CallFunction|DeathAnim))
    (:then_2
      (Input|DisableInput (Game|GetPlayerController 0) 0))
    (:then_3
      (Effects|SpawnEmitteratLocation (Variables|Inspector|GetDeathEmitter) (Transformation|GetActorLocation)))
    (:then_4
      (Audio|PlaySoundatLocation (.OutItem (Utilities|Array|Random (Variables|Inspector|GetDeathExplosionSound))) (Transformation|GetActorLocation) "0, 0, 0" 1.0 1.0 0.0 0 0 0 0))
    (:then_5
      (Utilities|FlowControl|Delay (Variables|Inspector|GetDeathDelay))
      (CallFunction|SetActiveVisual false))
    (:then_6
      (Default|CallEventPlayerDeath))))

(event EventTick
  (params (DeltaSeconds :type Float%20%28single-precision%29))
  ;[1 1 1] Update
  (Utilities|FlowControl|Sequence
    (:then_0
      (CallFunction|MoveForward))))

(event EventHit
  ;[1 0.317 0] Actions
  (if (Variables|Public|GetIsAlive)
    (Utilities|FlowControl|Sequence
      (:then_0
        (CallFunction|Death)))))

(event EventPickup
  (params (count :type Integer) (typePickup :type TypePickupEnum%20Enum :default "NewEnumerator0"))
  ;[1 0.317 0] Actions
  (if (Utilities|Enum|Equal(Enum) typePickup "NewEnumerator0")
    (bind _output_get (Variables|Public|SetYellowCoinsStored (+ count (Variables|Public|GetYellowCoinsStored))))
    (Development|PrintString (Utilities|String|ToString(Integer) _output_get))
    (elif (Utilities|Enum|Equal(Enum) typePickup "NewEnumerator1")
      (bind _output_get_2 (Variables|Public|SetBlueCoinsStores (+ count (Variables|Public|GetBlueCoinsStores))))
      (Development|PrintString (Utilities|String|ToString(Integer) _output_get_2)))))

(fn ConstructionScript)

(fn GetCharacterAnimRider
  (bind _asabp_run_character_rider (Utilities|Casting|CastToABP_RunCharacterRider (Components|SkeletalMesh|GetAnimInstance (Variables|Default|GetRider))))
  (return _asabp_run_character_rider))

(fn GetCharacterAnimHorse
  (params (Mesh :type Skeletal%20Mesh%20Component%20Object%20Reference))
  (bind _asabp_run_character_horse (Utilities|Casting|CastToABP_RunCharacterHorse (Components|SkeletalMesh|GetAnimInstance Mesh)))
  (return _asabp_run_character_horse))

(fn DeathAnim
  (Utilities|FlowControl|Sequence
    (:then_0
      (bind _abp (CallFunction|GetCharacterAnimHorse (Variables|Character|GetMesh)))
      (Default|DeathAnim _abp))
    (:then_1
      (bind _abp_2 (CallFunction|GetCharacterAnimHorse (Variables|Default|GetReins)))
      (Default|DeathAnim _abp_2))
    (:then_2
      (bind _abp_3 (CallFunction|GetCharacterAnimHorse (Variables|Default|GetSaddle)))
      (Default|DeathAnim _abp_3))
    (:then_3
      (bind _abp_4 (CallFunction|GetCharacterAnimHorse (Variables|Default|GetArmour)))
      (Default|DeathAnim _abp_4))
    (:then_4
      (bind _abp_5 (CallFunction|GetCharacterAnimRider))
      (Default|DeathAnim _abp_5))))

(fn SetActiveVisual
  (params (Value :type Boolean))
  (LocalVariables|Setvisibility Value)
  (Utilities|FlowControl|Sequence
    (:then_0
      (Rendering|SetVisibility (Variables|Character|GetMesh) (LocalVariables|Getvisibility) false))
    (:then_1
      (Rendering|SetVisibility (Variables|Default|GetReins) (LocalVariables|Getvisibility) false))
    (:then_2
      (Rendering|SetVisibility (Variables|Default|GetSaddle) (LocalVariables|Getvisibility) false))
    (:then_3
      (Rendering|SetVisibility (Variables|Default|GetRider) (LocalVariables|Getvisibility) false))
    (:then_4
      (Rendering|SetVisibility (Variables|Default|GetTail) (LocalVariables|Getvisibility) false))
    (:then_5
      (Rendering|SetVisibility (Variables|Default|GetArmour) (LocalVariables|Getvisibility) false))))