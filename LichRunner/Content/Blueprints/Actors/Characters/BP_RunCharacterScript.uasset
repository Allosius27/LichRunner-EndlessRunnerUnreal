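; Runner character Blueprint for a mounted rider on a horse, handling its randomized look and death feedback.
; The construction script applies a random material set to the horse, tack, armour and rider.
; BeginPlay assigns a player-death dispatcher, while OnDeath triggers death animations on each part's anim Blueprint, a hit emitter and a random explosion sound from a data table.
; DisableVisual hides all mesh parts.
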(event Custom|OnDeath
  (Utilities|FlowControl|Sequence
    (:then_0
      (Animations|DeathAnim))
    (:then_1
      (Effects|SpawnEmitteratLocation (Variables|Inspector|VisualEffects|GetHitEmitter) (Transformation|GetActorLocation)))
    (:then_2
      (Audio|PlaySoundatLocation (Sounds|GetAudioDataCue (.OutItem (Utilities|Array|Random (Variables|Inspector|Sounds|GetHitExplosionSounds)))) (Transformation|GetActorLocation) "0, 0, 0" 1.0 1.0 0.0 0 0 0 0))))

(event EventBeginPlay
  (Utilities|FlowControl|Sequence
    (:then_0
      (EventDispatchers|AssignDispatcheronPlayerDeath (EventDispatchers|CreateEvent :!event Custom|OnDeath)))))

(event EventDisableVisual
  (Character|SetActiveVisual false))

(fn ConstructionScript
  (Utilities|FlowControl|Sequence
    (:then_0
      (Character|SetMaterials (.OutItem (Utilities|Array|Random (Variables|Inspector|Character|GetCharacterMatsStructs)))))))

(fn GetAudioDataCue
  (params (SoundData :type Data%20Table%20Row%20Handle%20Structure))
  (bind (_datatable _rowname) (Utilities|Struct|BreakDataTableRowHandle SoundData))
  (bind _returnvalue (Utilities|GetDataTableRow _datatable _rowname)
    (:then
      _)
    (:RowNotFound
      _))
  (return (Utilities|Struct|BreakAudioStruct _returnvalue)))

(fn SetMaterials
  (params (matStruct :type Death%20Knight%20Materials%20Struct%20Structure))
  (LocalVariables|SetcurrentMatStruct matStruct)
  (Utilities|FlowControl|Sequence
    (:then_0
      (for _index (range 0 (- (Utilities|Array|Length (Rendering|Material|GetMaterials (Variables|Character|GetMesh))) 1))
        (Rendering|Material|SetMaterial (Variables|Character|GetMesh) _index (Utilities|Array|Get(acopy) (.horseMats (Utilities|Struct|BreakDeathKnightMaterialsStruct (LocalVariables|GetcurrentMatStruct))) _index))))
    (:then_1
      (Rendering|Material|SetMaterial (Variables|Components|GetReins) 0 (.armorMat (Utilities|Struct|BreakDeathKnightMaterialsStruct (LocalVariables|GetcurrentMatStruct))))
      (Rendering|Material|SetMaterial (Variables|Components|GetSaddle) 0 (.armorMat (Utilities|Struct|BreakDeathKnightMaterialsStruct (LocalVariables|GetcurrentMatStruct))))
      (Rendering|Material|SetMaterial (Variables|Components|GetArmour) 0 (.armorMat (Utilities|Struct|BreakDeathKnightMaterialsStruct (LocalVariables|GetcurrentMatStruct)))))
    (:then_2
      (Rendering|Material|SetMaterial (Variables|Components|GetRider) 0 (.riderMat (Utilities|Struct|BreakDeathKnightMaterialsStruct (LocalVariables|GetcurrentMatStruct)))))))

(fn GetCharacterAnimRider
  (bind _asabp_run_character_rider (Utilities|Casting|CastToABP_RunCharacterRider (Components|SkeletalMesh|GetAnimInstance (Variables|Components|GetRider))))
  (return _asabp_run_character_rider))

(fn GetCharacterAnimHorse
  (params (Mesh :type Skeletal%20Mesh%20Component%20Object%20Reference))
  (bind _asabp_run_character_horse (Utilities|Casting|CastToABP_RunCharacterHorse (Components|SkeletalMesh|GetAnimInstance Mesh)))
  (return _asabp_run_character_horse))

(fn DeathAnim
  (Utilities|FlowControl|Sequence
    (:then_0
      (bind _abp (Character|GetCharacterAnimHorse (Variables|Character|GetMesh)))
      (Default|DeathAnim _abp))
    (:then_1
      (bind _abp_2 (Character|GetCharacterAnimHorse (Variables|Components|GetReins)))
      (Default|DeathAnim _abp_2))
    (:then_2
      (bind _abp_3 (Character|GetCharacterAnimHorse (Variables|Components|GetSaddle)))
      (Default|DeathAnim _abp_3))
    (:then_3
      (bind _abp_4 (Character|GetCharacterAnimHorse (Variables|Components|GetArmour)))
      (Default|DeathAnim _abp_4))
    (:then_4
      (bind _abp_5 (Character|GetCharacterAnimRider))
      (Default|DeathAnim _abp_5))))

(fn SetActiveVisual
  (params (Value :type Boolean))
  (LocalVariables|Setvisibility Value)
  (Utilities|FlowControl|Sequence
    (:then_0
      (Rendering|SetVisibility (Variables|Character|GetMesh) (LocalVariables|Getvisibility) false))
    (:then_1
      (Rendering|SetVisibility (Variables|Components|GetReins) (LocalVariables|Getvisibility) false))
    (:then_2
      (Rendering|SetVisibility (Variables|Components|GetSaddle) (LocalVariables|Getvisibility) false))
    (:then_3
      (Rendering|SetVisibility (Variables|Components|GetRider) (LocalVariables|Getvisibility) false))
    (:then_4
      (Rendering|SetVisibility (Variables|Components|GetTail) (LocalVariables|Getvisibility) false))
    (:then_5
      (Rendering|SetVisibility (Variables|Components|GetArmour) (LocalVariables|Getvisibility) false))))