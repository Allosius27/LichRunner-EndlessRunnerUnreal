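; Base enemy character that chases the player, attacks and takes damage, with empty animation and attack-collider functions, apparently for children to override.
; Follow, Wait and Attack set states on BP_EnemyAIController, and following starts at BeginPlay.
; HitPlayer damages a living player, then disables attack colliders.
; StatsComponent dispatchers drive hit and death reactions: animation calls, a temporarily shown health bar and a damage-material flash using retriggerable delays.
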(event Custom|OnHit
  ;[1 0.3446 0] Take Damages
  (Utilities|FlowControl|Sequence
    (:then_0
      (bind _healthbar_ref (Variables|Public|UI|GetHealthBar_REF)
        (:then
          (Widget|SetVisibility _healthbar_ref "Visible")
          (Utilities|FlowControl|RetriggerableDelay (Variables|Inspector|UI|GetHeathBarVisibilityDelay))
          (Widget|SetVisibility (Variables|Public|UI|GetHealthBar_REF) "Collapsed"))
        (:else)))
    (:then_1
      (Animations|GetHitAnim))
    (:then_2
      (UI|UpdateHealthBar))
    (:then_3
      (Character|SetMeshMaterials (Variables|Inspector|Character|GetDamageMeshMaterials))
      (Utilities|FlowControl|RetriggerableDelay (Variables|Inspector|Character|GetDamageEffectDuration))
      (Character|SetMeshMaterials (Variables|Public|Character|GetBaseMeshMaterials)))))

(event Custom|OnDeath
  ;[1 0.3446 0] Take Damages
  (Utilities|FlowControl|Sequence
    (:then_0
      (Animations|DeathAnim))
    (:then_1
      (Widget|SetVisibility (Variables|Public|UI|GetHealthBar_REF) "Collapsed"))))

(event EventBeginPlay
  ;[1 1 1] Start
  (Utilities|FlowControl|Sequence
    (:then_0
      (bind _asbp_enemy_aicontroller (Utilities|Casting|CastToBP_EnemyAIController (AI|GetAIController self)))
      (Variables|Public|AI|SetEnemyAIController_REF _asbp_enemy_aicontroller))
    (:then_1
      (Class|Enemy|Follow (Game|GetPlayerCharacter 0)))
    (:then_2
      (EventDispatchers|BindEventtoDispatcheronDeath (Variables|Default|GetStatsComponent) (EventDispatchers|CreateEvent :!event Custom|OnDeath)))
    (:then_3
      (EventDispatchers|BindEventtoDispatcheronDamage (Variables|Default|GetStatsComponent) (EventDispatchers|CreateEvent :!event Custom|OnHit)))
    (:then_4
      (UI|InitAIHealthBarUI))
    (:then_5
      (Variables|Public|Character|SetBaseMeshMaterials (Rendering|Material|GetMaterials (Variables|Character|GetMesh))))))

(event EventAttack
  ;[0 0.08263 1] AI Behaviours
  (Default|SetEnemyState (Variables|Public|AI|GetEnemyAIController_REF) "NewEnumerator2")
  (Animations|AttackAnim))

(event Game|Damage|EventAnyDamage
  (params (Damage :type Float%20%28single-precision%29) (DamageType :type Damage%20Type%20Object%20Reference) (InstigatedBy :type Controller%20Object%20Reference) (DamageCauser :type Actor%20Object%20Reference))
  ;[1 0.3446 0] Take Damages
  (Class|Enemy|EnemyHit Damage))

(event EventFollow
  (params (followTarget :type Actor%20Object%20Reference))
  (bind _enemyaicontroller_ref (Variables|Public|AI|GetEnemyAIController_REF))
  ;[0 0.08263 1] AI Behaviours
  (if (Variables|/Script/LichRunner.StatsComponent|GetIsAlive (Variables|Default|GetStatsComponent))
    (Default|SetFollowActor _enemyaicontroller_ref followTarget)
    (Default|SetEnemyState _enemyaicontroller_ref "NewEnumerator1")))

(event EventWait
  ;[0 0.08263 1] AI Behaviours
  (Default|SetEnemyState (Variables|Public|AI|GetEnemyAIController_REF) "NewEnumerator0"))

(event EventHit
  (params (damages :type Float%20%28double-precision%29))
  ;[1 0.3446 0] Take Damages
  (if (Variables|/Script/LichRunner.StatsComponent|GetIsAlive (Variables|Default|GetStatsComponent))
    (Game|Damage|ApplyDamage self damages 0 0)))

(event EventHitPlayer
  (params (runCharacter :type Run%20Character%20Object%20Reference))
  ;[1 0.3446 0] Attack Actions
  (Utilities|IsValid runCharacter
    (:Is%20Valid
      (if (Variables|/Script/LichRunner.StatsComponent|GetIsAlive (Variables|/Script/LichRunner.RunCharacter|GetStatsComponent runCharacter))
        (bind _returnvalue (Class|Enemy|GetDamages))
        (Class|BPIHit|Hit(Message) runCharacter _returnvalue)
        (Actions|SetEnemyAttackCols false false false)))))

(fn ConstructionScript)

(fn AttackAnim)

(fn SetEnemyAttackCols
  (params (Value :type Boolean) (IsLeftAttack :type Boolean) (IsRightAttack :type Boolean)))

(fn DeathAnim)

(fn InitAIHealthBarUI
  (bind _asbpw_local_health_bar (Utilities|Casting|CastToBPW_LocalHealthBar (UserInterface|GetUserWidgetObject (Variables|Default|GetHealthBar))))
  (Variables|Public|UI|SetHealthBar_REF _asbpw_local_health_bar)
  (UI|UpdateHealthBar)
  (Widget|SetVisibility (Variables|Public|UI|GetHealthBar_REF) "Collapsed"))

(fn GetHitAnim)

(fn UpdateHealthBar
  (Variables|/Game/Blueprints/WidgetBlueprints/Core/BPW_LocalHealthBar.BPW_LocalHealthBar_C|SetMaxHealth (Variables|Public|UI|GetHealthBar_REF) (Variables|/Script/LichRunner.StatsComponent|GetMaxHealthPoints (Variables|Default|GetStatsComponent)))
  (Variables|/Game/Blueprints/WidgetBlueprints/Core/BPW_LocalHealthBar.BPW_LocalHealthBar_C|SetHealth (Variables|Public|UI|GetHealthBar_REF) (Variables|/Script/LichRunner.StatsComponent|GetHealthPoints (Variables|Default|GetStatsComponent))))

(fn SetMeshMaterials
  (params (Materials :type Array%20of%20Material%20Interface%20Object%20References))
  (LocalVariables|Set_materials Materials)
  (for (_ _array_index) (Rendering|Material|GetMaterials (Variables|Character|GetMesh))
    (if (Utilities|Array|IsValidIndex (LocalVariables|Get_materials) _array_index)
      (Rendering|Material|SetMaterial (Variables|Character|GetMesh) _array_index (Utilities|Array|Get(acopy) (LocalVariables|Get_materials) _array_index)))))