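; Item pickup actor that awards coins to the run character when collected.
; OnGet passes the pickup's coin count and type to the character's AddCoins, then plays a random pickup sound at the actor's location.
; A helper resolves the randomly chosen data table row handle into the sound asset, keeping audio cues data-driven.
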(event EventBeginPlay)

(event Collision|EventActorBeginOverlap
  (params (OtherActor :type Actor%20Object%20Reference)))

(event EventTick
  (params (DeltaSeconds :type Float%20%28single-precision%29)))

(event EventOnGet
  (params (runCharacter :type Run%20Character%20Object%20Reference))
  (Utilities|FlowControl|Sequence
    (:then_0
      (Class|RunCharacter|AddCoins runCharacter (Variables|Default|GetPickupCoinsCount) (Variables|Default|GetTypePickup)))
    (:then_1
      (Audio|PlaySoundatLocation (Sounds|GetAudioDataCue (.OutItem (Utilities|Array|Random (Variables|Inspector|Sounds|GetGetPickupSfx)))) (Transformation|GetActorLocation) "0, 0, 0" 1.0 1.0 0.0 0 0 0 0))))

(fn ConstructionScript)

(fn GetAudioDataCue
  (params (SoundData :type Data%20Table%20Row%20Handle%20Structure))
  (bind (_datatable _rowname) (Utilities|Struct|BreakDataTableRowHandle SoundData))
  (bind _returnvalue (Utilities|GetDataTableRow _datatable _rowname)
    (:then
      _)
    (:RowNotFound
      _))
  (return (Utilities|Struct|BreakAudioStruct _returnvalue)))