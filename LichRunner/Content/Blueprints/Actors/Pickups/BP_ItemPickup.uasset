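; BP_ItemPickup is a pickup actor that the running character collects by touching it.
; Overlap on its PickupTrigger component casts the other actor to BP_RunCharacter and passes it to Collect, ignoring any other actor.
; Collect reports the pickup's count and type to the character through PickupMessage, plays a pickup sound at its location, then destroys itself.
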(event OnComponentBeginOverlap(PickupTrigger)
  (params (OverlappedComponent :type Primitive%20Component%20Object%20Reference) (OtherActor :type Actor%20Object%20Reference) (OtherComp :type Primitive%20Component%20Object%20Reference) (OtherBodyIndex :type Integer) (bFromSweep :type Boolean) (SweepResult :type Hit%20Result%20Structure%20%28by%20ref%29))
  ;[1 1 1] Collisions Management
  (bind _asbp_run_character (Utilities|Casting|CastToBP_RunCharacter OtherActor))
  (CallFunction|Collect _asbp_run_character))

(fn ConstructionScript)

(fn Collect
  (params (runCharacter :type BP%20Run%20Character%20Object%20Reference))
  (Utilities|FlowControl|Sequence
    (:then_0
      (Class|BPIHit|Pickup(Message) runCharacter (Variables|Inspector|GetPickupCount) (Variables|Inspector|GetTypePickup)))
    (:then_1
      (Audio|PlaySoundatLocation (Variables|Inspector|GetGetPickupSfx) (Transformation|GetActorLocation) "0, 0, 0" 1.0 1.0 0.0 0 0 0 0))
    (:then_2
      (Actor|DestroyActor))))