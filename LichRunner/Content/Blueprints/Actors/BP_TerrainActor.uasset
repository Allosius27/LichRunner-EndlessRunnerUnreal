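; BP_TerrainActor is a terrain actor that carries an attached prefab and exposes an attach point.
; On BeginPlay it attaches a valid Prefab actor to itself, keeping the prefab's world transform.
; Every Tick it passes itself to CallEventCheckTerrainDistance for a terrain distance check, whose logic lives outside this graph.
; GetAttachTransform returns the world transform of its AttachPoint component.
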(event EventBeginPlay
  (bind _prefab (Variables|Inspector|GetPrefab)
    (:then
      (Transformation|AttachActorToActor _prefab self "None" "KeepWorld" "KeepWorld" "KeepWorld" true))
    (:else)))

(event EventTick
  (params (DeltaSeconds :type Float%20%28single-precision%29))
  (Utilities|FlowControl|Sequence
    (:then_0
      (Default|CallEventCheckTerrainDistance self))))

(fn ConstructionScript)

(fn GetAttachTransform
  (return (Transformation|GetWorldTransform (Variables|Default|GetAttachPoint))))