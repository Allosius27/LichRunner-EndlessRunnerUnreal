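; Floor tile for a runner game that fills itself with random obstacles and pickups and exposes an attach point transform.
; Construction makes weighted rolls to add random child actor classes at random points inside spawn trigger boxes.
; BP_RunCharacter overlapping the end trigger fires the exited event, and Tick fires a player-distance check while HasLifeTime is false.
; TileExit destroys the tile after a delay.
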(event OnComponentBeginOverlap(EndPosTrigger)
  (params (OverlappedComponent :type Primitive%20Component%20Object%20Reference) (OtherActor :type Actor%20Object%20Reference) (OtherComp :type Primitive%20Component%20Object%20Reference) (OtherBodyIndex :type Integer) (bFromSweep :type Boolean) (SweepResult :type Hit%20Result%20Structure%20%28by%20ref%29))
  ;[1 1 1] Collisions Management
  (Utilities|Casting|CastToBP_RunCharacter OtherActor)
  (Development|PrintString (Utilities|GetDisplayName self))
  (Default|CallEventExitedbyPlayer self))

(event Custom|TileExit
  ;[1 1 1] State Management
  (Utilities|FlowControl|Delay (Variables|Inspector|GetLifeTimeTooFarPlayer))
  (Actor|DestroyActor))

(event EventTick
  (params (DeltaSeconds :type Float%20%28single-precision%29))
  ;[1 1 1] Update
  (Utilities|FlowControl|Sequence
    (:then_0
      (if (not (Variables|Public|GetHasLifeTime))
        (Default|CallEventCheckDistancetoPlayer self)))))

(fn ConstructionScript
  (Utilities|FlowControl|Sequence
    (:then_0
      (CallFunction|SpawnObstacle (Variables|Inspector|GetObstacleSpawnRandomWeight)))
    (:then_1
      (for _index (range 0 (Variables|Inspector|GetPickupsToSpawnCount))
        (CallFunction|SpawnPickup (Variables|Inspector|GetPickupSpawnRandomWeight))))))

(fn GetAttachTransform
  (return (Transformation|GetWorldTransform (Variables|Default|GetAttachPoint))))

(fn SpawnObstacle
  (params (randomWeight :type Float%20%28double-precision%29))
  (bind _spawnobstaclestrigger (Variables|Default|GetSpawnObstaclesTrigger))
  (bind _obstacles (Variables|Inspector|GetObstacles))
  (if (and (Math|Random|RandomBoolwithWeight randomWeight) (Variables|Public|GetCanCreateObstacles))
    (bind _returnvalue (AddComponent|AddChildActorComponent true (Math|Transform|MakeTransform (Math|Random|RandomPointinBoundingBox (Transformation|GetWorldLocation _spawnobstaclestrigger) (Variables|/Script/Engine.BoxComponent|GetBoxExtent _spawnobstaclestrigger)))))
    (ChildActorComponent|SetChildActorClass _returnvalue (Utilities|Array|Get(acopy) _obstacles (Math|Random|RandomInteger (Utilities|Array|Length _obstacles))))))

(fn SpawnPickup
  (params (RandomWeight :type Float%20%28double-precision%29))
  (bind _spawnpickupstrigger (Variables|Default|GetSpawnPickupsTrigger))
  (bind _pickups (Variables|Inspector|GetPickups))
  (if (and (Math|Random|RandomBoolwithWeight RandomWeight) (Variables|Public|GetCanCreatePickups))
    (bind _returnvalue (AddComponent|AddChildActorComponent true (Math|Transform|MakeTransform (Math|Random|RandomPointinBoundingBox (Transformation|GetWorldLocation _spawnpickupstrigger) (Variables|/Script/Engine.BoxComponent|GetBoxExtent _spawnpickupstrigger)))))
    (ChildActorComponent|SetChildActorClass _returnvalue (Utilities|Array|Get(acopy) _pickups (Math|Random|RandomInteger (Utilities|Array|Length _pickups))))))