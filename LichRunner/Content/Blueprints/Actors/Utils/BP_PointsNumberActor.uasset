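; BP_PointsNumberActor is a short-lived floating points number that pops up and flies off in the world.
; On BeginPlay it passes PointsAmount to its BPW_FloatingPoints widget and launches its static mesh with a random upward, sideways-scattered impulse that ignores mass.
; The actor destroys itself when the widget signals that its lifetime is over.
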(event Custom|WidgetDeath
  (Actor|DestroyActor))

(event EventBeginPlay
  (bind _asbpw_floating_points (Utilities|Casting|CastToBPW_FloatingPoints (UserInterface|GetUserWidgetObject (Variables|Default|GetWidget))))
  (EventDispatchers|BindEventtoWidgetLifeTimeOver _asbpw_floating_points (delegate Custom|WidgetDeath))
  (Class|BPInterfaceSetPointsValue|SetPointsValue(Message) _asbpw_floating_points (Variables|Default|GetPointsAmount))
  (Physics|AddImpulse (Variables|Default|GetStaticMesh) (Math|Vector|MakeVector (Math|Random|RandomFloatinRange -2e+02 2e+02) (Math|Random|RandomFloatinRange -2e+02 2e+02) (Math|Random|RandomFloatinRange 2e+02 4e+02)) "None" true))

(fn ConstructionScript)