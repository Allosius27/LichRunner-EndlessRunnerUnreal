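; Obstacle actor for what appears to be a runner game, reacting when the player's BP_RunCharacter hits it.
; The collider's hit event filters for that character and passes it to OnHit.
; OnHit sends HitMessage to the character, spawns a particle effect and plays a random explosion sound at the obstacle's location.
; GetAudioDataCue resolves that sound from a data table row handle.
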(event OnComponentHit(ObstacleCollider)
  (params (HitComponent :type Primitive%20Component%20Object%20Reference) (OtherActor :type Actor%20Object%20Reference) (OtherComp :type Primitive%20Component%20Object%20Reference) (NormalImpulse :type Vector :default "0, 0, 0") (Hit :type Hit%20Result%20Structure%20%28by%20ref%29))
  ;[1 1 1] Collisions Management
  (bind _asbp_run_character (Utilities|Casting|CastToBP_RunCharacter OtherActor))
  (CallFunction|OnHit _asbp_run_character))

(fn ConstructionScript)

(fn OnHit
  (params (runCharacter :type BP%20Run%20Character%20Object%20Reference))
  (Utilities|FlowControl|Sequence
    (:then_0
      (Class|BPIHit|Hit(Message) runCharacter))
    (:then_1
      (Effects|SpawnEmitteratLocation (Variables|Inspector|GetHitEmitter) (Transformation|GetActorLocation)))
    (:then_2
      (Audio|PlaySoundatLocation (CallFunction|GetAudioDataCue (.OutItem (Utilities|Array|Random (Variables|Inspector|GetHitExplosionSounds)))) (Transformation|GetActorLocation) "0, 0, 0" 1.0 1.0 0.0 0 0 0 0))))

(fn GetAudioDataCue
  (params (SoundData :type Data%20Table%20Row%20Handle%20Structure))
  (bind (_datatable _rowname) (Utilities|Struct|BreakDataTableRowHandle SoundData))
  (bind _returnvalue (Utilities|GetDataTableRow _datatable _rowname)
    (:then
      _)
    (:RowNotFound
      _))
  (return (Utilities|Struct|BreakAudioStruct _returnvalue)))