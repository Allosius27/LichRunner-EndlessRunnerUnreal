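; Game mode for an endless runner that sets up floor tiles, coin display, music and terrain, and reloads the level after a delay on game over.
; Floor tiles chain from each one's attach transform, and each exited tile spawns a successor, with obstacles left off the initial batch.
; Terrain actors are recycled: those the player passes move to the front-most attach point, and the list is re-sorted by X.
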(event Custom|OnTileExited
  (params (tile :type BP%20Floor%20Tile%20Object%20Reference))
  ;[1 0.317 0] Tiles Actions
  (CallFunction|CreateTile true true)
  (Default|TileExit tile))

(event Custom|GameOver
  ;[1 0 0.7962] Global Management
  (Utilities|FlowControl|Delay (Variables|Inspector|GetRestartLevelDelay))
  (bind _returnvalue (Game|GetCurrentLevelName true))
  (Game|OpenLevel(byName) (Utilities|String|StringToName _returnvalue)))

(event EventBeginPlay
  ;[1 1 1] Init
  (Utilities|FlowControl|Sequence
    (:then_0
      (Game|GetPlayerController))
    (:then_1
      (|InitTiles))
    (:then_2
      (|InitUI))
    (:then_3
      (|InitMusic))
    (:then_4
      (|InitTerrainsActors))))

(fn ConstructionScript)

(fn CreateTile
  (params (TileCanCreatePickups :type Boolean) (TileCanCreateObstacles :type Boolean))
  (bind _returnvalue (Game|SpawnActorfromClass "/Game/Blueprints/Actors/BP_FloorTile.BP_FloorTile_C" (Variables|Public|GetCurrentSpawnPoint) "Undefined" 0 TileCanCreatePickups TileCanCreateObstacles 0))
  (bind _attachtransform (Default|GetAttachTransform _returnvalue))
  (Variables|Public|SetCurrentSpawnPoint _attachtransform)
  (EventDispatchers|BindEventtoEventExitedbyPlayer _returnvalue (EventDispatchers|CreateEvent :!event Custom|OnTileExited))
  (EventDispatchers|BindEventtoEventCheckDistancetoPlayer _returnvalue (EventDispatchers|CreateEvent :!event Custom|CheckTileDistanceToPlayer)))

(fn GetAudioDataCue
  (params (SoundData :type Data%20Table%20Row%20Handle%20Structure))
  (bind (_datatable _rowname) (Utilities|Struct|BreakDataTableRowHandle SoundData))
  (bind _returnvalue (Utilities|GetDataTableRow _datatable _rowname)
    (:then
      _)
    (:RowNotFound
      _))
  (return (Utilities|Struct|BreakAudioStruct _returnvalue)))

(fn TerrainDistanceComparator
  (params (ObjectA :type Object%20Object%20Reference) (ObjectB :type Object%20Object%20Reference))
  (bind _asbp_terrain_actor (Utilities|Casting|CastToBP_TerrainActor ObjectA))
  (LocalVariables|SetterrainActorA _asbp_terrain_actor)
  (bind _asbp_terrain_actor_2 (Utilities|Casting|CastToBP_TerrainActor ObjectB))
  (LocalVariables|SetterrainActorB _asbp_terrain_actor_2)
  (return (< (.x (Transformation|GetActorLocation (LocalVariables|GetterrainActorA))) (.x (Transformation|GetActorLocation (LocalVariables|GetterrainActorB))))))

(event Custom|CheckTileDistanceToPlayer
  (params (Tile :type BP%20Floor%20Tile%20Object%20Reference)))

(event Custom|CheckTerrainActorDistance
  (params (terrain :type BP%20Terrain%20Actor%20Object%20Reference))
  (bind _terrainactors (Variables|Public|GetTerrainActors))
  (bind _playercontroller_ref (Variables|Public|GetPlayerController_REF)
    (:then
      (bind _runcharacter (Variables|/Game/Blueprints/Controllers/BP_RunPlayerController.BP_RunPlayerController_C|GetRunCharacter _playercontroller_ref)
        (:then
          (if (and (> (.x (Transformation|GetActorLocation _runcharacter)) (+ (.x (Transformation|GetActorLocation terrain)) (Variables|/Game/Blueprints/Actors/BP_TerrainActor.BP_TerrainActor_C|GetDistanceAcceptance terrain))) (Utilities|Array|IsNotEmpty (Variables|Public|GetTerrainActors)))
            (Transformation|SetActorLocation terrain (.location (Default|GetAttachTransform (Utilities|Array|Get(acopy) _terrainactors (- (Utilities|Array|Length _terrainactors) 1)))) false false)
            (Class|LowEntryExtendedStandardLibrary|SortObjectArrayDirectly (Variables|Public|GetTerrainActors) (EventDispatchers|CreateEvent :!event TerrainDistanceComparator) false)))
        (:else)))
    (:else)))